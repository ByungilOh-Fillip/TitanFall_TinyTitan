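; BP_UIKar98 is an animated Kar98 actor, apparently a display piece for UI, that spins and moves vertically.
; Each Tick adds local yaw from RotSpeed scaled by DeltaSeconds.
; It also samples a float Curve at scaled game time and adds the result to its current Z.
; That vertical offset accumulates per frame without delta-time scaling, so the motion depends on frame rate.
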(event EventBeginPlay)

(event Collision|EventActorBeginOverlap
  (params (OtherActor :type Actor%20Object%20Reference)))

(event EventTick
  (params (DeltaSeconds :type Float%20%28single-precision%29))
  (bind _returnvalue (Transformation|GetActorLocation))
  ;[0.15 0.15 0.15 0.5] move kar98
  (Utilities|FlowControl|Sequence
    (:then_0
      (Transformation|AddActorLocalRotation (Math|Rotator|MakeRotator 0.0 0.0 (* DeltaSeconds (Variables|Default|GetrotSpeed))) false false))
    (:then_1
      (Transformation|SetActorLocation (Math|Vector|MakeVector (.x _returnvalue) (.y _returnvalue) (+ (.z _returnvalue) (* (Math|Curves|GetFloatValue (Variables|Default|Getcurve) (* (Utilities|Time|GetGameTimeinSeconds) 0.4)) 5.0))) false false))))

(fn ConstructionScript)