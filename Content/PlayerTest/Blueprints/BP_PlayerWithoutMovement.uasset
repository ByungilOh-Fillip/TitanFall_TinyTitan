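; First-person player test pawn with Enhanced Input look, double jump, hitscan fire and breath control.
; Each tick computes camera-relative velocity with custom gravity and a downward ground trace, but the SetActorLocation applying it is disconnected.
; A sine offset sways the camera; holding breath stills it, then triggers a shake if held too long.
; Firing traces from the camera, spawning a bullet-hole decal and timed shake, gated by IsStoped.
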(event Input|EnhancedActionEvents|EnhancedInputActionIA_Jump
  (params (ActionValue :type Float%20%28double-precision%29) (ElapsedSeconds :type Float%20%28double-precision%29) (TriggeredSeconds :type Float%20%28double-precision%29) (InputAction :type Input%20Action%20Object%20Reference :default "/Game/PlayerTest/Inputs/IA_Jump.IA_Jump"))
  ;[0.1284 0.3316 0.09048 0.5] Move to velocity
  ;;[0.15 0.15 0.15 0.5] Restrict Jump Count ( JumpCount <2 )
  (:Started
    (if (< (Variables|Default|GetJumpCount) 2)
      (Variables|Default|SetJumpCount (+ 1 (Variables|Default|GetJumpCount)))
      (Variables|Default|SetZ_Velocity (Variables|Default|GetJumpPower))
      (Variables|Default|SetIsGrounded false))))

(event Input|EnhancedActionEvents|EnhancedInputActionIA_Fire
  (params (ActionValue :type Boolean) (ElapsedSeconds :type Float%20%28double-precision%29) (TriggeredSeconds :type Float%20%28double-precision%29) (InputAction :type Input%20Action%20Object%20Reference :default "/Game/PlayerTest/Inputs/IA_Fire.IA_Fire"))
  (bind _camera (Variables|Default|GetCamera))
  (bind _returnvalue (Transformation|GetSocketLocation _camera "None"))
  ;[0.07465 0.07465 0.07465 0.5] Fire & CameraShake & SpawnDecal
  (:Started
    (if (stale _output_get)
      (bind _outhit (Collision|LineTraceByChannel _returnvalue (+ _returnvalue (* (Math|Vector|GetForwardVector _camera) (Variables|Default|GetShootRange))) "TraceTypeQuery1" false 0 "ForDuration"))
      (bind _returnvalue_2 (CameraShakes|StartCameraShake (Game|GetPlayerCameraManager 0) "/Game/PlayerTest/Blueprints/BP_CameraShake.BP_CameraShake_C" 1.5 "CameraLocal" "0, 0, 0"))
      (Utilities|FlowControl|Sequence
        (:then_0
          (bind _output_get (Variables|Default|SetIsStoped false))
          (bind _returnvalue_3 (Rendering|Decal|SpawnDecalatLocation "/Game/PlayerTest/Materials/M_BulletHole.M_BulletHole" "15.000000,15.000000,15.000000" (.location _outhit) (Math|Rotator|MakeRotfromX (.impactnormal _outhit)) 3e+01))
          (Rendering|Components|Decal|SetFadeScreenSize _returnvalue_3 0.01))
        (:then_1
          (Utilities|FlowControl|RetriggerableDelay 0.7)
          (CameraShakes|StopCameraShake (Game|GetPlayerCameraManager 0) _returnvalue_2 true)))
      (else
        (Utilities|FlowControl|Delay 0.4)
        (Variables|Default|SetIsStoped true)))))

(event Input|EnhancedActionEvents|EnhancedInputActionIA_BreathControl
  (params (ActionValue :type Float%20%28double-precision%29) (ElapsedSeconds :type Float%20%28double-precision%29) (TriggeredSeconds :type Float%20%28double-precision%29) (InputAction :type Input%20Action%20Object%20Reference :default "/Game/PlayerTest/Inputs/IA_BreathControl.IA_BreathControl"))
  ;[0.15 0.15 0.15 0.5] Breath Control
  (:Triggered
    (if (> ElapsedSeconds 2.0)
      (Variables|Default|SetBreath 0.0)
      (if (> ElapsedSeconds 1e+01)
        (Utilities|FlowControl|DoOnce false :!label _label
          (:Completed
            (bind _returnvalue (CameraShakes|StartCameraShake (Game|GetPlayerCameraManager 0) "/Game/PlayerTest/Blueprints/BP_CameraShake.BP_CameraShake_C" 0.7 "CameraLocal" "0, 0, 0"))
            (Utilities|FlowControl|RetriggerableDelay 4.0)
            (CameraShakes|StopCameraShake (Game|GetPlayerCameraManager 0) _returnvalue true)
            (Variables|Default|SetBreath 0.2)
            (goto _label Reset))))))
  (:Canceled
    (Variables|Default|SetBreath 0.2)))

(event EventBeginPlay
  ;[0.4774 0.4359 0 0.5] Begin Actor
  (bind _asplayer_controller (Utilities|Casting|CastToPlayerController (Pawn|GetController)))
  (Input|AddMappingContext (PlayerController|LocalPlayerSubsystems|GetEnhancedInputLocalPlayerSubsystem _asplayer_controller) "/Game/PlayerTest/Inputs/IMC_PlayerInput.IMC_PlayerInput" 0 "(bIgnoreAllPressedKeysUntilRelease=True,bForceImmediately=False,bNotifyUserSettings=False)"))

(event Collision|EventActorBeginOverlap
  (params (OtherActor :type Actor%20Object%20Reference)))

(event EventTick
  (params (DeltaSeconds :type Float%20%28single-precision%29))
  (bind _returnvalue (Transformation|GetActorLocation))
  (bind _returnvalue_2 (Transformation|GetActorLocation))
  (bind _returnvalue_3 (Input|EnhancedActionValues|GetIA_Look))
  ;[0.1284 0.3316 0.09048 0.5] Move to velocity
  (CallFunction|BreathCycle)
  (CallFunction|SettoFeet)
  (CallFunction|ControlPawnYaw (.x _returnvalue_3))
  (CallFunction|ControlCameraPitch (.y _returnvalue_3))
  (CallFunction|CarculateZVelocity)
  (CallFunction|PlayerMove)
  (bind _returnvalue_4 (Collision|LineTraceByChannel _returnvalue_2 (+ _returnvalue_2 (Variables|Default|GettoFeet)) "TraceTypeQuery1" false 0 "None"))
  (Variables|Default|SetIsGrounded _returnvalue_4)
  (Rendering|Debug|DrawDebugLine _returnvalue_2 (Math|Vector|MakeVector (.x _returnvalue) (.y _returnvalue) (Variables|Default|GetZ_Velocity)) "(R=0.939236,G=0.003287,B=0.008087,A=1.000000)" 0.0 0.0))

(fn ConstructionScript)

(fn PlayerMove
  (bind _returnvalue (Input|EnhancedActionValues|GetIA_Player))
  (bind _camera (Variables|Default|GetCamera))
  ;[0.15 0.15 0.15 0.5] Move & Jump
  (Variables|Default|SetDirection (+ (* (Math|Vector|GetForwardVector _camera) (.x _returnvalue)) (* (.y _returnvalue) (Math|Vector|GetRightVector _camera))))
  (Variables|Default|SetVelocity (Math|Vector|MakeVector (.x (* (Variables|Default|GetDirection) (Variables|Gravity|GetSpeed))) (.y (* (Variables|Default|GetDirection) (Variables|Gravity|GetSpeed))) (Variables|Default|GetZ_Velocity))))

(fn CarculateZVelocity
  ;[0 0.1847 0.7691 0.113] Z_Velocity Carculate
  (if (and (Variables|Default|GetIsGrounded) (<= (Variables|Default|GetZ_Velocity) 0.0))
    (Variables|Default|SetZ_Velocity 0.0)
    (Variables|Default|SetJumpCount 0)
    (else
      (Variables|Default|SetZ_Velocity (- (Variables|Default|GetZ_Velocity) (* (Variables|Gravity|GetGravity) (Utilities|Time|GetWorldDeltaSeconds))))
      (Variables|Default|SetIsGrounded false)
      (Variables|Default|SetZ_Velocity (- (Variables|Default|GetZ_Velocity) (* (Variables|Default|GetWeight) (Utilities|Time|GetWorldDeltaSeconds)))))))

(fn SettoFeet
  ;[0.15 0.15 0.15 0.5] Actor의 길이의 절반을 구한 후 LineTrace 길이 설정
  (Variables|Default|SettoFeet (Math|Vector|MakeVector 0.0 0.0 (+ (/ (* (.z (Transformation|GetActorScale3D)) -1e+02) 2.0) -1e+01))))

(fn ControlPawnYaw
  (params (C :type Float%20%28double-precision%29))
  (Pawn|Input|AddControllerYawInput (* C (Variables|Default|GetInterpSpeed) (Utilities|Time|GetWorldDeltaSeconds))))

(fn ControlCameraPitch
  (params (A :type Float%20%28double-precision%29))
  (bind _output_get (Variables|Default|SetCurPitch (* A (Utilities|Time|GetWorldDeltaSeconds) (Variables|Default|GetInterpSpeed) -1.0)))
  (if (Math|Float|InRange(Float) _output_get -8e+01 8e+01)
    (Pawn|Input|AddControllerPitchInput (Variables|Default|GetCurPitch))))

(fn BreathCycle
  (Transformation|AddLocalOffset (Variables|Default|GetCamera) (Math|Vector|MakeVector 0.0 0.0 (* (Math|Trig|Sin(Radians) (* (Utilities|Time|GetGameTimeinSeconds) 3.14)) (Variables|Default|GetBreath))) false false))