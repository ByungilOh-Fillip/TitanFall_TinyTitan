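; BP_SaveGame provides save and load functions for a score value, apparently the player's best score.
; SaveScoreData creates a new BP_SaveGame object, sets its ScoreData and writes it to the "BestScoreData" slot.
; LoadScoreData checks that a save exists, loads and casts it, then returns ScoreData.
; Loading uses an empty slot name, so it does not read the slot that saving writes.
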(fn SaveScoreData
  (params (SaveValue :type Integer))
  (bind _returnvalue (SaveGame|CreateSaveGameObject "BP_SaveGame_C"))
  (bind _output_get (Variables|Default|SetSaveInstance _returnvalue))
  (Variables|BP_SaveGame_C|SetScoreData _output_get SaveValue)
  (SaveGame|SaveGametoSlot _output_get "BestScoreData"))

(fn LoadScoreData
  (params (BestScore :type Integer))
  (SaveGame|DoesSaveGameExist)
  (if true
    (bind _returnvalue (SaveGame|LoadGamefromSlot))
    (bind _asbp_save_game (Utilities|Casting|CastToBP_SaveGame _returnvalue))
    (return (Variables|BP_SaveGame_C|GetScoreData _asbp_save_game))))